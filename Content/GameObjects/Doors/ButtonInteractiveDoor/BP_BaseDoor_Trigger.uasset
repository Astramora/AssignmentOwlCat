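; BP_BaseDoor_Trigger is a child door Blueprint with two animated panels and a state indicator.
; Its construction script runs the parent's, then registers the left and right door parts with DoorAnimationComponent.
; On BeginPlay it binds to OnStateChanged to set the indicator material, with both Closed and Opened applying the closed-indicator material.
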(event `self.ReceiveBeginPlay`
  (add `self.OnStateChanged` (delegate `ChangeIndicatorColor`)))

(event `ChangeIndicatorColor` :!signature `self.OnStateChanged`
  (params (NewState :type "EDoorState Enum" :default "Closed"))
  (switch `EDoorState` NewState
    (:`Closed`
      _)
    (:`Opened`
      _))
  (`PrimitiveComponent.SetMaterial` (`self.Indicator`) 0 "/Game/GameObjects/Doors/Materials/M_Door_IndicatorClosed.M_Door_IndicatorClosed"))

(fn `UserConstructionScript`
  (`parent.UserConstructionScript`)
  (`TimelineAnimationComponent.SetAnimatedComponents` (`self.DoorAnimationComponent`) (`|MakeArray` (`self.DoorPartLeft`) (`self.DoorPartRight`) :!type "SceneComponent Object Reference")))