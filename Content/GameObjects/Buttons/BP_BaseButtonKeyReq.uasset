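; Base button that requires a key, unlocking when an interacting player character holds the matching key type.
; On interaction start, it casts the actor to BP_PlayerCharacter and checks for KeyReq, then enables itself and switches the button mesh to the interactable material.
; The construction script runs the parent's setup and registers ButtonMesh with the ButtonAnimationComponent for animation.
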(event `InteractionInterface.StartInteraction`
  (params (OtherActor :type "Actor Object Reference"))
  (bind _asbp_player_character (cast `/Game/Core/PlayerCharacter/BP_PlayerCharacter` OtherActor))
  (if (`KeyringLibrary.ActorHasKey` _asbp_player_character (`self.KeyReq`))
    (`self.SetIsEnabled` true)
    (`PrimitiveComponent.SetMaterial` (`self.ButtonMesh`) 0 "/Game/GameObjects/Materials/MI_Interactable.MI_Interactable")))

(fn `UserConstructionScript`
  (`parent.UserConstructionScript`)
  (`TimelineAnimationComponent.SetAnimatedComponents` (`self.ButtonAnimationComponent`) (`|MakeArray` (`self.ButtonMesh`) :!type "SceneComponent Object Reference")))