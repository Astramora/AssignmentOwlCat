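; Construction-script generator that builds a pipe along the actor's spline from repeated spline mesh components.
; It divides the spline into sectors sized by MeshLength times the actor's X scale, leaving any remainder shorter than one sector uncovered.
; Each X-forward segment has collision disabled and takes local start and end points from the spline, with tangents clamped to sector length to match each piece.
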(fn `UserConstructionScript`
  (bind _returnvalue_x (`KismetMathLibrary.BreakVector` (`self.GetActorScale3D`)))
  (bind _spline (`self.Spline`))
  (bind _spline_2 (`self.Spline`))
  (set `self.SectorLength` (* _returnvalue_x (`self.MeshLength`)))
  (for _index (range (`KismetMathLibrary.FTrunc` (/ (`SplineComponent.GetSplineLength` (`self.Spline`)) (`self.SectorLength`))))
    (bind _returnvalue (`AddComponent|NODE_AddSplineMeshComponent-0`))
    (`SplineMeshComponent.SetForwardAxis` _returnvalue "X" true)
    (`PrimitiveComponent.SetCollisionEnabled` _returnvalue "NoCollision")
    (bind _returnvalue_2 (* _index (`self.SectorLength`)))
    (bind _returnvalue_3 (* (+ _index 1) (`self.SectorLength`)))
    (`SplineMeshComponent.SetStartAndEnd` _returnvalue (`SplineComponent.GetLocationAtDistanceAlongSpline` _spline_2 _returnvalue_2 "Local") (`KismetMathLibrary.ClampVectorSize` (`SplineComponent.GetTangentAtDistanceAlongSpline` _spline_2 _returnvalue_2 "Local") 0.0 (`self.SectorLength`)) (`SplineComponent.GetLocationAtDistanceAlongSpline` _spline _returnvalue_3 "Local") (`KismetMathLibrary.ClampVectorSize` (`SplineComponent.GetTangentAtDistanceAlongSpline` _spline _returnvalue_3 "Local") 0.0 (`self.SectorLength`)) true)))