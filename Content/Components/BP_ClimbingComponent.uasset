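; Player character component that automatically vaults the player onto ledges while falling.
; On Tick, a forward sphere trace finds a wall, a second finds the ledge, and the target is offset forward from it.
; If capsule overlap and trace checks find clear space, the character lerps there, with a bound climb-end event resetting state.
; GetCanVault, GetStartEndVaultTrace and SetTargetLocation are unused in these graphs.
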(event `self.ReceiveBeginPlay`
  (bind _asbp_player_character (cast `/Game/Core/PlayerCharacter/BP_PlayerCharacter` (`self.GetOwner`)))
  (bind _output_get (set `self.BP Player Character` _asbp_player_character))
  (add `/Game/Core/PlayerCharacter/BP_PlayerCharacter.ClimbEnd` _output_get (`|CreateDelegate` :!event `EndClimb`)))

(event `self.ReceiveTick`
  (params (DeltaSeconds :type "Float (single-precision)"))
  (if (and (`NavMovementComponent.IsFalling` (`Character.CharacterMovement` (`self.BP Player Character`))) (not (`self.IsVaulting`)))
    (`self.SwitchOnClimbState`
      (:`NotClimbing`
        (bind (_wallhitlocation _waswallhit) (`self.WallTrace`))
        (if _waswallhit
          (bind _wasledgehit (`self.LedgeTrace` _wallhitlocation))
          (if _wasledgehit
            (`self.CalculateTargetLocation`)
            (if (and (`self.CheckSpaceOnLedge` (`self.TargetLocation`)) (`self.CheckObstacles`))
              (`self.StartClimb`))))))))

(event `StartClimb`
  (set `self.IsVaulting` true)
  (set `self.CurrentClimbState` "NewEnumerator0")
  (`/Game/Core/PlayerCharacter/BP_PlayerCharacter.LerpPlayerLocation` (`self.BP Player Character`) (`self.TargetLocation`) (/ 1.0 (`self.VaultSpeed`))))

(event `EndClimb`
  (set `self.CurrentClimbState` "NewEnumerator1")
  (set `self.IsVaulting` false))

(fn `CalculateTargetLocation`
  (set `self.TargetLocation` (`KismetMathLibrary.MakeVector` (+ (.x (`self.Ledge Location`)) (.x (* (`Actor.GetActorForwardVector` (`self.BP Player Character`)) (`self.VaultDepth`)))) (+ (.y (`self.Ledge Location`)) (.y (* (`Actor.GetActorForwardVector` (`self.BP Player Character`)) (`self.VaultDepth`)))) (+ (.z (`self.Ledge Location`)) (`CapsuleComponent.GetScaledCapsuleHalfHeight` (`Character.CapsuleComponent` (`self.BP Player Character`)))))))

(fn `CheckCapsuleCollision`
  (params (Center :type "Vector Structure") (Radius :type "Float (double-precision)") (HalfHeight :type "Float (double-precision)"))
  (returns (`IsCapsuleCollided?` :type Boolean))
  (bind (_outactors _returnvalue) (`KismetSystemLibrary.CapsuleOverlapActors` Center Radius HalfHeight (`|MakeArray` "ObjectTypeQuery1" "ObjectTypeQuery2" "ObjectTypeQuery3" :!type "EObjectTypeQuery Enum") null (`|MakeArray` (`self.BP Player Character`) :!type "Actor Object Reference")))
  (return _returnvalue))

(fn `CheckObstacles`
  (returns (ReturnValue :type Boolean))
  (bind _bp_player_character (`self.BP Player Character`))
  (bind (_outhit _returnvalue) (`KismetSystemLibrary.CapsuleTraceSingle` (+ (* (`Actor.GetActorUpVector` _bp_player_character) 230.0) (`Actor.K2_GetActorLocation` _bp_player_character)) (`self.TargetLocation`) 44.0 44.0 "TraceTypeQuery1"))
  (return (not _returnvalue)))

(fn `CheckSpaceOnLedge`
  (params (HitLocation :type "Vector Structure"))
  (returns (IsSpaceAvailable :type Boolean))
  (bind _capsulecomponent (`Character.CapsuleComponent` (`self.BP Player Character`)))
  (return (not (`self.CheckCapsuleCollision` (+ HitLocation (0.0 0.0 22.0)) (`CapsuleComponent.GetScaledCapsuleRadius` _capsulecomponent) (`CapsuleComponent.GetScaledCapsuleHalfHeight` _capsulecomponent)))))

(fn `GetCanVault`
  (returns (CanVault :type Boolean))
  (return false))

(fn `GetStartEndVaultTrace`
  (returns (StartLoc :type "Vector Structure") (EndLoc :type "Vector Structure"))
  (bind _bp_player_character (`self.BP Player Character`))
  (bind _returnvalue (`CapsuleComponent.GetScaledCapsuleHalfHeight` (`Character.CapsuleComponent` _bp_player_character)))
  (bind _returnvalue_2 (+ (`Actor.K2_GetActorLocation` _bp_player_character) (* (`Actor.GetActorForwardVector` _bp_player_character) (`self.VaultTraceLength`))))
  (return (+ _returnvalue_2 (`KismetMathLibrary.MakeVector` 0.0 0.0 _returnvalue)) (- _returnvalue_2 (`KismetMathLibrary.MakeVector` 0.0 0.0 _returnvalue))))

(fn `LedgeTrace`
  (params (WallHitLocation :type "Vector Structure"))
  (returns (WasLedgeHit :type Boolean))
  (bind (_outhit _returnvalue) (`KismetSystemLibrary.SphereTraceSingle` (+ WallHitLocation (0.0 0.0 20.0)) WallHitLocation 40.0 "TraceTypeQuery1"))
  (set `self.Ledge Location` (`.Location` (`GameplayStatics.BreakHitResult` _outhit)))
  (return _returnvalue))

(fn `SetTargetLocation`
  (bind (_impactpoint_x _impactpoint_y) (`KismetMathLibrary.BreakVector` (`self.ImpactPoint`)))
  (bind (_returnvalue_x _returnvalue_y _returnvalue_z) (`KismetMathLibrary.BreakVector` (`Actor.K2_GetActorLocation` (`self.BP Player Character`))))
  (bind _returnvalue (+ (`KismetMathLibrary.MakeVector` _impactpoint_x _impactpoint_y (- _returnvalue_z 45.0)) (* (0.0 0.0 0.0) (`self.VaultDepth`))))
  (bind (_outhit _returnvalue_2) (`KismetSystemLibrary.SphereTraceSingle` (+ _returnvalue (0.0 0.0 120.0)) _returnvalue 30.0 "TraceTypeQuery1"))
  (if (and _returnvalue_2 (`CharacterMovementComponent.IsWalkable` (`Character.CharacterMovement` (`self.BP Player Character`)) _outhit))
    (set `self.TargetLocation` (`KismetMathLibrary.MakeVector` (.x (`.Location` (`GameplayStatics.BreakHitResult` _outhit))) (.y (`.Location` (`GameplayStatics.BreakHitResult` _outhit))) (+ (.z (`.Location` (`GameplayStatics.BreakHitResult` _outhit))) (`CapsuleComponent.GetScaledCapsuleHalfHeight` (`Character.CapsuleComponent` (`self.BP Player Character`))))))))

(fn `WallTrace`
  (returns (WallHitLocation :type "Vector Structure") (WasWallHit :type Boolean))
  (bind _bp_player_character (`self.BP Player Character`))
  (bind _returnvalue (`Actor.K2_GetActorLocation` _bp_player_character))
  (bind (_outhit _returnvalue_2) (`KismetSystemLibrary.SphereTraceSingle` :`Start` _returnvalue :`End` (+ _returnvalue (* (`Actor.GetActorForwardVector` _bp_player_character) (`self.VaultTraceLength`))) :`Radius` 20.0 :`TraceChannel` "TraceTypeQuery1" :`DrawTime` 2.0))
  (return (`.Location` (`GameplayStatics.BreakHitResult` _outhit)) _returnvalue_2))